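; BP_EnergyShield is an energy shield that can be raised, lowered and rotated around its parent component's pivot.
; Enable and disable events toggle visibility and use timelines to grow or flatten the mesh's Z scale, switching collision to query-only or off on completion.
; Q/E or gamepad shoulder buttons set direction flags.
; Tick applies yaw to the parent by a fixed RotationSpeed step per frame, without delta-time scaling.
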(event `Enable shield`
  (`SceneComponent.ToggleVisibility` (`self.EnergyShield`) false)
  (bind (_direction _scale) (`Timeline|Timeline_0` :!via `PlayFromStart`)
    (:`Update`
      (`SceneComponent.SetRelativeScale3D` (`self.EnergyShield`) (`KismetMathLibrary.VLerp` (0.75 0.75 0.0) (0.75 0.75 0.75) _scale)))
    (:`Finished`
      (`PrimitiveComponent.SetCollisionEnabled` (`self.EnergyShield`) "QueryOnly"))))

(event `self.ReceiveBeginPlay`
  (`self.EnableInput` (`GameplayStatics.GetPlayerController` 0))
  (set `self.Init scale` (`SceneComponent.RelativeScale3D` (`self.EnergyShield`))))

(event `Disable Sheild`
  (bind (_init_scale_x _init_scale_y _init_scale_z) (`KismetMathLibrary.BreakVector` (`self.Init scale`)))
  (bind (_direction _scale) (`Timeline|Scale` :!via `PlayFromStart`)
    (:`Update`
      (`SceneComponent.SetRelativeScale3D` (`self.EnergyShield`) (`KismetMathLibrary.VLerp` (`KismetMathLibrary.MakeVector` _init_scale_x _init_scale_y _init_scale_z) (`KismetMathLibrary.MakeVector` _init_scale_x _init_scale_y 0.001) _scale)))
    (:`Finished`
      (`SceneComponent.ToggleVisibility` (`self.EnergyShield`) false)
      (`PrimitiveComponent.SetCollisionEnabled` (`self.EnergyShield`) "NoCollision"))))

(event `Key|Gamepad_LeftShoulder`
  (params (Key :type "Key Structure"))
  ;[1 1 1] Rotate Shield Around Player
  (:`Pressed`
    (set `self.RotateShieldLeft` true :!label _label))
  (:`Released`
    (set `self.RotateShieldLeft` false :!label _label_2)))

(event `Key|Q`
  (params (Key :type "Key Structure"))
  ;[1 1 1] Rotate Shield Around Player
  (:`Pressed`
    (goto _label))
  (:`Released`
    (goto _label_2)))

(event `self.ReceiveTick`
  (params (DeltaSeconds :type "Float (single-precision)"))
  (bind _parent (`self.Parent`))
  ;[1 1 1] Rotate Shield Around Player
  (`|ExecutionSequence`
    (:`then_0`
      (if (`self.RotateShieldLeft`)
        (`SceneComponent.K2_AddLocalRotation` _parent (`KismetMathLibrary.MakeRotator` 0.0 0.0 (* (`self.RotationSpeed`) -1.0)) false false)))
    (:`then_1`
      (if (`self.RotateShieldRight`)
        (`SceneComponent.K2_AddLocalRotation` _parent (`KismetMathLibrary.MakeRotator` 0.0 0.0 (`self.RotationSpeed`)) false false)))))

(event `Key|E`
  (params (Key :type "Key Structure"))
  ;[1 1 1] Rotate Shield Around Player
  (:`Pressed`
    (set `self.RotateShieldRight` true :!label _label_3))
  (:`Released`
    (set `self.RotateShieldRight` false :!label _label_4)))

(event `Key|Gamepad_RightShoulder`
  (params (Key :type "Key Structure"))
  ;[1 1 1] Rotate Shield Around Player
  (:`Pressed`
    (goto _label_3))
  (:`Released`
    (goto _label_4)))

(event `self.EnergyShield.OnComponentHit`
  (params (HitComponent :type "PrimitiveComponent Object Reference") (OtherActor :type "Actor Object Reference") (OtherComp :type "PrimitiveComponent Object Reference") (NormalImpulse :type "Vector Structure") (Hit :type "HitResult Structure (by ref)")))

(fn `UserConstructionScript`)